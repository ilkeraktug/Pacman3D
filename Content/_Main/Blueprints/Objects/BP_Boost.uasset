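; BP_Boost is a collectible boost pickup that notifies the game mode when the player picks it up.
; Tick spins the Boost component steadily around its Z axis.
; A SphereCollision overlap uses a message call on the other actor to confirm it is the player, then destroys the pickup.
; It then gets the game mode reference through another message and calls BoostCollected, leaving the boost effect outside this Blueprint.
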(event OnComponentBeginOverlap(SphereCollision)
  (params (OverlappedComponent :type Primitive%20Component%20Object%20Reference) (OtherActor :type Actor%20Object%20Reference) (OtherComp :type Primitive%20Component%20Object%20Reference) (OtherBodyIndex :type Integer) (bFromSweep :type Boolean) (SweepResult :type Hit%20Result%20Structure%20%28by%20ref%29))
  ;[1 1 1] Collecting boost logic
  (bind _playerref (Class|INTPlayer|PlayerRef(Message) OtherActor))
  (Utilities|IsValid _playerref
    (:Is%20Valid
      (Actor|DestroyActor)
      (bind _gamemode (Class|INTGamemode|GamemodeRef(Message) (Game|GetGameMode)))
      (Default|CallBoostCollected _gamemode))))

(event EventBeginPlay
  (|CallParentFunction) ; This node is disabled and will not be called.\nDrag off pins to build functionality.
)

(event Collision|EventActorBeginOverlap
  (params (OtherActor :type Actor%20Object%20Reference))
  (|CallParentFunction OtherActor) ; This node is disabled and will not be called.\nDrag off pins to build functionality.
)

(event EventTick
  (params (DeltaSeconds :type Float%20%28single-precision%29))
  (bind _boost (Variables|Default|GetBoost))
  (bind _relativerotation (Variables|/Script/Engine.SceneComponent|GetRelativeRotation _boost))
  ;[1 1 1] Rotate on Z axis
  (|CallParentFunction DeltaSeconds)
  (Transformation|SetWorldRotation _boost (Math|Rotator|MakeRotator (.roll _relativerotation) (.pitch _relativerotation) (+ (.yaw _relativerotation) (* DeltaSeconds 9e+01))) false false))

(fn ConstructionScript
  (|CallParentFunction))