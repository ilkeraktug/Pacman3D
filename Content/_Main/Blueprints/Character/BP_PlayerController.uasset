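; Player controller that routes input for movement, look, lantern, camera view and pausing to the controlled character.
; On BeginPlay it caches the pawn and gets a player reference through a message call.
; Movement follows control yaw; key presses flip-flop the light and lantern equip state or cycle three camera states.
; Scrolling adjusts a lit lantern's intensity within clamped limits, and Escape pauses the game and opens the pause menu widget.
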(event EventBeginPlay
  ;[1 1 1] Init variables
  (bind _output_get (Variables|Controller|SetControllerPawn (Pawn|GetControlledPawn)))
  (bind _playerref (Class|INTPlayer|PlayerRef(Message) _output_get))
  (Variables|M_Ref|SetPlayer%20Ref _playerref))

(event Input|ActionEvents|InputActionEqiupLantern
  (params (Key :type Key%20Structure :default "None"))
  (bind _player_ref (Variables|M_Ref|GetPlayer%20Ref))
  ;[1 1 1] Equip Lantern
  (:Pressed
    (Utilities|FlowControl|FlipFlop
      (:A
        (Variables|/Game/_Main/Blueprints/Character/PlayerCharacter.PlayerCharacter_C|SetisLanternEquiped _player_ref true))
      (:B
        (Variables|/Game/_Main/Blueprints/Character/PlayerCharacter.PlayerCharacter_C|SetisLanternEquiped _player_ref false)))))

(event Input|ActionEvents|InputActionToggleLight
  (params (Key :type Key%20Structure :default "None"))
  (bind _player_ref (Variables|M_Ref|GetPlayer%20Ref))
  ;[1 1 1] Toggle Light
  (:Pressed
    (Utilities|FlowControl|FlipFlop
      (:A
        (Default|EnableLight _player_ref true))
      (:B
        (Default|EnableLight _player_ref false)))))

(event Input|ActionEvents|InputActionChangeView
  (params (Key :type Key%20Structure :default "None"))
  (bind _player_ref (Variables|M_Ref|GetPlayer%20Ref))
  ;[1 1 1] Change Camera
  (:Pressed
    (Variables|/Game/_Main/Blueprints/Character/PlayerCharacter.PlayerCharacter_C|SetcameraState _player_ref (Class|KismetMathLibrary|PercentByteByte (+ (Variables|/Game/_Main/Blueprints/Character/PlayerCharacter.PlayerCharacter_C|GetcameraState _player_ref) 1) 3))
    (Default|SetCamera _player_ref)))

(event Input|AxisEvents|InputAxisMoveForward
  (params (AxisValue :type Float%20%28single-precision%29))
  (bind _controllerpawn (Variables|Controller|GetControllerPawn))
  ;[1 1 1] Move
  (Utilities|IsValid _controllerpawn
    (:Is%20Valid
      (Pawn|Input|AddMovementInput (Variables|Controller|GetControllerPawn) (Math|Vector|GetForwardVector (Math|Rotator|MakeRotator 0.0 0.0 (.yaw (Pawn|GetControlRotation _controllerpawn :!class /Script/Engine.Pawn)))) AxisValue false))))

(event Input|AxisEvents|InputAxisMoveRight
  (params (AxisValue :type Float%20%28single-precision%29))
  (bind _controllerpawn (Variables|Controller|GetControllerPawn))
  ;[1 1 1] Move
  (Utilities|IsValid _controllerpawn
    (:Is%20Valid
      (Pawn|Input|AddMovementInput (Variables|Controller|GetControllerPawn) (Math|Vector|GetRightVector (Math|Rotator|MakeRotator 0.0 0.0 (.yaw (Pawn|GetControlRotation _controllerpawn :!class /Script/Engine.Pawn)))) AxisValue false))))

(event Input|AxisEvents|InputAxisLookUp
  (params (AxisValue :type Float%20%28single-precision%29))
  ;[1 1 1] Mouse Inputs
  (Class|PlayerController|AddPitchInput AxisValue))

(event Input|AxisEvents|InputAxisTurn
  (params (AxisValue :type Float%20%28single-precision%29))
  ;[1 1 1] Mouse Inputs
  (Class|PlayerController|AddYawInput AxisValue))

(event Input|AxisEvents|InputAxisSetting_LightIntensity
  (params (AxisValue :type Float%20%28single-precision%29))
  ;[1 1 1] Change light intensity with mouse scroll
  (bind _lantern (Default|GetLantern (Variables|M_Ref|GetPlayer%20Ref)))
  (if (Variables|/Game/_Main/Blueprints/Objects/BP_Lantern.BP_Lantern_C|GetisLightOn _lantern)
    (Default|SetLightIntensity _lantern (Math|Float|Clamp(Float) (+ (Variables|/Game/_Main/Blueprints/Objects/BP_Lantern.BP_Lantern_C|GetLightIntensity _lantern) (* AxisValue (Variables|Default|GetInstensityChangeEveryScroll))) 2.5e+02 3e+03))))

(event Input|KeyboardEvents|Escape
  (params (Key :type Key%20Structure :default "None"))
  ;[1 1 1] Pause Menu
  (:Pressed
    (Game|SetGamePaused true)
    (Variables|Default|SetbShowMouseCursor true)
    (bind _returnvalue (UserInterface|CreateWidget "/Game/_Main/Blueprints/UI/Widget_PauseMenu.Widget_PauseMenu_C"))
    (UserInterface|Viewport|AddtoViewport _returnvalue 0)))

(fn ConstructionScript)

(fn PlayerControllerRef
  (return self))