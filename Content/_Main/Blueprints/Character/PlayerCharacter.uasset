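; Player character for a coin-collecting maze-style game, with switchable first-person, third-person and top-view cameras and a hand-attached lantern spawned at BeginPlay.
; Gamemode events drive life loss, which respawns the player at PlayerStart with a visibility flicker, and fruit boosts, which flicker the lantern light faster near expiry.
; Tick checks score and lives to show pausing win or lose screens, and toggles a looping footstep-sound timer based on horizontal velocity.
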(event Custom|LostLife_Event
  (bind _player_flick_rate (Variables|PlayerFlick|GetPlayer%20Flick%20Rate))
  ;[1 1 1] Lose a life event
  (CallFunction|LoseLife)
  (Audio|PlaySound2D "/Game/_Main/Blueprints/Sounds/Death_SoundCue.Death_SoundCue" 1.0 1.0 0.0 0 0)
  (Transformation|SetActorLocation (Transformation|GetActorLocation (Variables|/Game/_Main/Blueprints/BP_Gamemode.BP_Gamemode_C|GetPlayerStart (Variables|M_Ref|GetGamemode))) false false)
  ;[0.1413 0 0.4072] Player Respawn Flick Effect
  (Variables|M_State|SetisPlayerFlicking true)
  (Rendering|SetActorHiddenInGame true :!label _label)
  (Utilities|FlowControl|Delay _player_flick_rate)
  (Rendering|SetActorHiddenInGame false)
  (Utilities|FlowControl|Sequence
    (:then_0
      (Utilities|FlowControl|DoOnce false :!label _label_2
        (:Completed
          (Utilities|FlowControl|Delay (Variables|PlayerFlick|GetPlayerFlickDuration))
          (Variables|M_State|SetisPlayerFlicking false)
          (goto _label_2 Reset))))
    (:then_1
      (Utilities|FlowControl|Delay _player_flick_rate)
      (if (Variables|M_State|GetisPlayerFlicking)
        (goto _label)))))

(event Custom|BoostCollected_Event
  ;[1 0.01967 0.1173] Setting up boost activated/collected events
  (Default|CallBoostActived (Variables|M_Ref|GetGamemode))
  (Audio|PlaySound2D "/Game/_Main/Blueprints/Sounds/EatFruit_SoundCue.EatFruit_SoundCue" 1.0 1.0 0.0 0 0)
  (Variables|M_State|SetisBoosted true)
  (bind _asbp_lantern (Utilities|Casting|CastToBP_Lantern (Variables|M_SpawnObject|GetLantern)))
  ;[0.3504 0 1] Light Flick Effect
  (Rendering|SetVisibility (Variables|/Game/_Main/Blueprints/Objects/BP_Lantern.BP_Lantern_C|GetPointLight _asbp_lantern) false false :!label _label)
  (Utilities|FlowControl|Delay (Variables|BoostTimeSettings|GetLightFlickDuration))
  (Rendering|SetVisibility (Variables|/Game/_Main/Blueprints/Objects/BP_Lantern.BP_Lantern_C|GetPointLight _asbp_lantern) true false)
  ;[1 0 0.667] Set timer for deactive boost
  (Utilities|FlowControl|Sequence
    (:then_0
      (Utilities|FlowControl|DoOnce false :!label _label_2
        (:Completed
          (Utilities|FlowControl|Delay (- (Variables|BoostTimeSettings|GetBoostDuration) (Variables|BoostTimeSettings|GetBoostLastSeconds)))
          ;[1 1 1] Change Flickering rate to indicate boost is about to be deactived.
          (Variables|BoostTimeSettings|SetLightFlickDuration 0.1)
          (Utilities|FlowControl|Delay (Variables|BoostTimeSettings|GetBoostDuration))
          (Variables|M_State|SetisBoosted false)
          (Default|CallBoostDeactived (Variables|M_Ref|GetGamemode))
          (Variables|BoostTimeSettings|SetLightFlickDuration 0.35)
          (goto _label_2 Reset))))
    (:then_1
      (Utilities|FlowControl|Delay (Variables|BoostTimeSettings|GetLightFlickDuration))
      (if (Variables|M_State|GetisBoosted)
        (goto _label)))))

(event Custom|PlayFootStepSound
  ;[1 1 1] Foot Step Sound
  (Audio|PlaySoundatLocation "/Game/_Main/Blueprints/Sounds/FootStep_SoundCue.FootStep_SoundCue" (Transformation|GetActorLocation) "0, 0, 0" 1.0 1.0 0.0 0 0 0))

(event EventBeginPlay
  (bind _mesh (Variables|Character|GetMesh))
  ;[1 0.01185 0] Create & Attach lantern to hand
  (|CallParentFunction)
  (Utilities|FlowControl|Sequence
    (:then_0
      ;[1 0.02819 0] Make Camera Array and Set them inactive
      (bind _output_get (Variables|M_Array|SetCameraArray (Utilities|Array|MakeArray (Variables|Default|GetFirstPersonCamera) (Variables|Default|GetThirdPersonCamera) (Variables|Default|GetTop-View%20Camera))))
      (for _array_element _output_get
        (Components|Activation|SetActive _array_element false false))
      (CallFunction|SetCamera))
    (:then_1
      (bind _returnvalue (Game|SpawnActorfromClass (Variables|SpawnObjects|GetLanternClass) (Transformation|GetWorldTransform _mesh) "AlwaysSpawn" 0 0))
      (bind _output_get_2 (Variables|M_SpawnObject|SetLantern _returnvalue))
      (Transformation|AttachComponentToComponent _output_get_2 _mesh (Variables|SpawnObjects|GetLantern%20Socket) "SnapToTarget" "SnapToTarget" "SnapToTarget" true))
    (:then_2
      (bind _playercontrollerref (Class|INTPlayerController|PlayerControllerRef(Message) (Game|GetPlayerController 0)))
      (Variables|M_Ref|SetPlayerController _playercontrollerref))
    (:then_3
      ;[1 1 1] Lose a life event
      (bind _gamemode (Class|INTGamemode|GamemodeRef(Message) (Game|GetGameMode)))
      (Utilities|IsValid _gamemode
        (:Is%20Valid
          (bind _output_get_3 (Variables|M_Ref|SetGamemode _gamemode))
          (EventDispatchers|BindEventtoLostLife _output_get_3 (delegate Custom|LostLife_Event)))))
    (:then_4
      ;[1 0.01967 0.1173] Setting up boost activated/collected events
      (EventDispatchers|BindEventtoBoostCollected _output_get_3 (delegate Custom|BoostCollected_Event)))))

(event EventTick
  (params (DeltaSeconds :type Float%20%28single-precision%29))
  (bind _returnvalue (Transformation|GetVelocity))
  ;[1 1 1] Checks if game is over
  (Utilities|FlowControl|Sequence
    (:then_0
      (if (== (Variables|M_State|GetScore) (Variables|M_State|GetMaxCoin))
        (CallFunction|GameWon)))
    (:then_1
      (if (== (Variables|M_State|GetLifeCount) 0)
        (CallFunction|GameLost)))
    (:then_2
      ;[1 1 1] Foot Step Sound
      (if (Math|Boolean|ORBoolean (> (.x _returnvalue) 1.0) (< (.x _returnvalue) -1.0) (> (.y _returnvalue) 1.0) (< (.y _returnvalue) -1.0))
        (Utilities|FlowControl|DoOnce false :!label _label
          (:Completed
            (bind _returnvalue_2 (Utilities|Time|SetTimerbyEvent (delegate Custom|PlayFootStepSound) (Variables|SoundParameters|GetFootStep%20Interval) true))))
        (else
          (Utilities|Time|ClearandInvalidateTimerbyHandle _returnvalue_2)
          (goto _label Reset))))))

(fn ConstructionScript
  (|CallParentFunction))

(fn EnableLight
  (params (EnableLight :type Boolean))
  (bind _asbp_lantern (Utilities|Casting|CastToBP_Lantern (Variables|M_SpawnObject|GetLantern)))
  (Default|EnableLight _asbp_lantern EnableLight))

(fn SetCamera
  (bind _cameraarray (Variables|M_Array|GetCameraArray))
  (for _array_element _cameraarray
    (Components|Activation|SetActive _array_element false false)
    (Components|Activation|SetActive (Utilities|Array|Get(acopy) _cameraarray (Math|Conversions|ToInteger(Byte) (Variables|M_State|GetcameraState))) true false)))

(fn GetArrowCompenent
  (return (Variables|Default|GetPointCoin)))

(fn GetLantern
  (bind _asbp_lantern (Utilities|Casting|CastToBP_Lantern (Variables|M_SpawnObject|GetLantern)))
  (return _asbp_lantern))

(fn LoseLife
  (Variables|M_State|SetLifeCount (- (Variables|M_State|GetLifeCount) 1)))

(fn GameWon
  (Viewport|RemoveAllWidgets)
  (bind _returnvalue (UserInterface|CreateWidget (Variables|Widget|GetGameWon_Widget)))
  (UserInterface|Viewport|AddtoViewport _returnvalue 0)
  (Variables|/Script/Engine.PlayerController|SetbShowMouseCursor (Variables|M_Ref|GetPlayerController) true)
  (Game|SetGamePaused true))

(fn GameLost
  (Viewport|RemoveAllWidgets)
  (bind _returnvalue (UserInterface|CreateWidget (Variables|Widget|GetGameLost_Widget)))
  (UserInterface|Viewport|AddtoViewport _returnvalue 0)
  (Variables|/Script/Engine.PlayerController|SetbShowMouseCursor (Variables|M_Ref|GetPlayerController) true)
  (Game|SetGamePaused true))

(fn PlayerRef
  (return self))