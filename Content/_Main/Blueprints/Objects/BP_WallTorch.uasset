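; BP_WallTorch is a wall torch object that reacts when the player enters its box collision.
; On overlap, an interface-style PlayerRefMessage call on the other actor must return a valid reference before anything happens.
; It then plays the torch sound at its location and runs a timeline that rolls the Cube mesh while setting the point light to the LightIntensity value.
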(event OnComponentBeginOverlap(BoxCollision)
  (params (OverlappedComponent :type Primitive%20Component%20Object%20Reference) (OtherActor :type Actor%20Object%20Reference) (OtherComp :type Primitive%20Component%20Object%20Reference) (OtherBodyIndex :type Integer) (bFromSweep :type Boolean) (SweepResult :type Hit%20Result%20Structure%20%28by%20ref%29))
  (bind _cube (Variables|Default|GetCube))
  (bind _relativerotation (Variables|/Script/Engine.SceneComponent|GetRelativeRotation _cube))
  (bind _playerref (Class|INTPlayer|PlayerRef(Message) OtherActor))
  (Utilities|IsValid _playerref
    (:Is%20Valid
      (Audio|PlaySoundatLocation "/Game/_Main/Blueprints/Sounds/WallTorch_SoundCue.WallTorch_SoundCue" (Transformation|GetActorLocation) "0, 0, 0" 1.0 1.0 0.0 0 0 0)
      (bind _rotation_angle_x (Timeline|RollAngleTimeline Play)
        (:Update
          (Transformation|SetRelativeRotation (Variables|Default|GetCube) (Math|Rotator|MakeRotator _rotation_angle_x (.pitch _relativerotation) (.yaw _relativerotation)) false false)
          (Rendering|Components|Light|SetIntensity (Variables|Default|GetPointLight) (Variables|Default|GetLight%20Intensity)))))))

(event EventBeginPlay
  (|CallParentFunction) ; This node is disabled and will not be called.\nDrag off pins to build functionality.
)

(event Collision|EventActorBeginOverlap
  (params (OtherActor :type Actor%20Object%20Reference))
  (|CallParentFunction OtherActor) ; This node is disabled and will not be called.\nDrag off pins to build functionality.
)

(event EventTick
  (params (DeltaSeconds :type Float%20%28single-precision%29))
  (|CallParentFunction DeltaSeconds) ; This node is disabled and will not be called.\nDrag off pins to build functionality.
)

(fn ConstructionScript
  (|CallParentFunction))