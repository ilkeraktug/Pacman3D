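; Pac-Man-style enemy that hunts the player and becomes killable while the game mode's boost is active.
; Boost events toggle chase/flee flags and swap randomly colored normal and see-through materials.
; Tick drives AI moves to random navigable points around the player, or back to base for a delayed respawn after death.
; Player hits either kill it for score or cost a life; movement starts a looping zombie-sound timer.
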(event OnComponentHit(CapsuleComponent)
  (params (HitComponent :type Primitive%20Component%20Object%20Reference) (OtherActor :type Actor%20Object%20Reference) (OtherComp :type Primitive%20Component%20Object%20Reference) (NormalImpulse :type Vector :default "0, 0, 0") (Hit :type Hit%20Result%20Structure%20%28by%20ref%29))
  (bind _player_ref (Variables|Default|GetPlayer%20Ref))
  ;[1 1 1] Determines whos gonna hurt. Player or the Enemy
  (if (== OtherActor (Variables|Default|GetPlayer%20Ref))
    (if (Variables|Default|GetcanDie)
      (Variables|M_State|SetisGoingBase true)
      (Rendering|SetVisibility (Variables|Default|GetBody) false false)
      (Utilities|FlowControl|DoOnce false
        (:Completed
          (bind _output_get (Variables|/Game/_Main/Blueprints/Character/PlayerCharacter.PlayerCharacter_C|SetEnemyKillScore _player_ref (+ (Variables|/Game/_Main/Blueprints/Character/PlayerCharacter.PlayerCharacter_C|GetEnemyKillScore _player_ref) 2)))
          (Development|PrintString (Utilities|String|ToString(Integer) _output_get))))
      (else
        (bind _gamemode (Class|INTGamemode|GamemodeRef(Message) (Game|GetGameMode)))
        (Utilities|IsValid _gamemode
          (:Is%20Valid
            (Default|CallLostLife _gamemode)))))))

(event Custom|BoostDeactived_Event
  ;[1 0.01306 0] Setting up events
  (CallFunction|BoostDeactivated)
  (CallFunction|DisableSeeThrough))

(event Custom|BoostActived_Event
  ;[1 0.01306 0] Setting up events
  (CallFunction|BoostActivated)
  (CallFunction|EnableSeeThrough))

(event Custom|PlayFootStepSound
  ;[1 1 1] Zombie Sound
  (Audio|PlaySoundatLocation "/Game/_Main/Blueprints/Sounds/Enemy_SoundCue.Enemy_SoundCue" (Transformation|GetActorLocation) "0, 0, 0" 1.0 1.0 0.0 0 0 0))

(event EventBeginPlay
  (bind _gamemode (Variables|Default|GetGamemode))
  ;[1 0.01306 0] Setting up events
  (|CallParentFunction)
  (EventDispatchers|BindEventtoBoostDeactived _gamemode (delegate Custom|BoostDeactived_Event))
  (EventDispatchers|BindEventtoBoostActived _gamemode (delegate Custom|BoostActived_Event)))

(event EventTick
  (params (DeltaSeconds :type Float%20%28single-precision%29))
  (bind _returnvalue (Transformation|GetVelocity))
  (bind _player_ref (Variables|Default|GetPlayer%20Ref))
  (Utilities|FlowControl|Sequence
    (:then_0
      (if (Variables|M_State|GetisGoingBase)
        ;[1 1 1] Enemy is going base to respawn.
        (Variables|/Script/Engine.CharacterMovementComponent|SetMaxWalkSpeed (Variables|Character|GetCharacterMovement) (Variables|AISettings|GetGoingBaseSpeed))
        (Utilities|FlowControl|DoOnce false :!label _label
          (:Completed
            (AI|AIMoveTo self (Variables|/Game/_Main/Blueprints/BP_Gamemode.BP_Gamemode_C|GetEnemyBaseLocation (Variables|Default|GetGamemode)) 0 5.0 false
              (:then
                (if (Math|Vector|Equal(Vector) (Variables|/Game/_Main/Blueprints/BP_Gamemode.BP_Gamemode_C|GetEnemyBaseLocation (Variables|Default|GetGamemode)) (Transformation|GetActorLocation) 1e+02)
                  (Utilities|FlowControl|Delay (Variables|AISettings|GetRespawnTime))
                  (Variables|M_State|SetisGoingBase false)
                  (Variables|Default|SetcanDie false)
                  (Rendering|SetVisibility (Variables|Default|GetBody) true false)
                  ;[1 1 1] Determines whos gonna hurt. Player or the Enemy
                  (Utilities|FlowControl|DoOnce false) ; enters at Reset
                ))
              (:OnSuccess
                (Utilities|FlowControl|Delay (Math|Random|RandomFloatinRange 0.1 0.4) :!label _label_2)
                (goto _label Reset))
              (:OnFail
                (goto _label_2)))))
        (else
          ;[1 1 1] Enemy is chasing player..
          (if (Variables|Default|GetisChasing)
            (Variables|/Script/Engine.CharacterMovementComponent|SetMaxWalkSpeed (Variables|Character|GetCharacterMovement) (Variables|AISettings|GetChasingSpeed))
            (Utilities|FlowControl|DoOnce false :!label _label_3
              (:Completed
                (bind (_randomlocation _returnvalue_2) (Class|NavigationSystemV1|GetRandomLocationinNavigableRadius (Transformation|GetActorLocation (Variables|Default|GetPlayer%20Ref)) (Variables|AISettings|GetChasingRadius) 0 0))
                (if _returnvalue_2
                  (AI|AIMoveTo self _randomlocation 0 1.0 false
                    (:then
                      _)
                    (:OnSuccess
                      _)
                    (:OnFail
                      _))
                  (Utilities|FlowControl|Delay (Math|Random|RandomFloatinRange 0.5 1.0))
                  (goto _label_3 Reset))))
            (else
              ;[1 1 1] Boost is activated and enemy is going random.
              (if (Variables|Default|GetisRunningAway)
                (Variables|/Script/Engine.CharacterMovementComponent|SetMaxWalkSpeed (Variables|Character|GetCharacterMovement) (Variables|AISettings|GetChasingSpeed))
                (Utilities|FlowControl|DoOnce false :!label _label_4
                  (:Completed
                    (bind (_randomlocation_2 _returnvalue_3) (Class|NavigationSystemV1|GetRandomLocationinNavigableRadius (Transformation|GetActorLocation (Variables|Default|GetPlayer%20Ref)) (Variables|AISettings|GetRunawayRadius) 0 0))
                    (if _returnvalue_3
                      (AI|AIMoveTo self _randomlocation_2 0 1.0 false
                        (:then
                          _)
                        (:OnSuccess
                          _)
                        (:OnFail
                          _))
                      (Utilities|FlowControl|Delay (Math|Random|RandomFloatinRange 0.5 1.0))
                      (goto _label_4 Reset))))))))))
    (:then_1
      ;[1 1 1] Zombie Sound
      (if (Math|Boolean|ORBoolean (> (.x _returnvalue) 1.0) (< (.x _returnvalue) -1.0) (> (.y _returnvalue) 1.0) (< (.y _returnvalue) -1.0))
        (Utilities|FlowControl|DoOnce false :!label _label_5
          (:Completed
            (bind _returnvalue_4 (Utilities|Time|SetTimerbyEvent (delegate Custom|PlayFootStepSound) (Variables|SFX|GetZombie%20Sound%20Interval) true))))
        (else
          (Utilities|Time|ClearandInvalidateTimerbyHandle _returnvalue_4)
          (goto _label_5 Reset))))))

(fn ConstructionScript
  (|CallParentFunction)
  (Variables|Default|SetisRunningAway false)
  (Variables|Default|SetcanDie false)
  (Variables|Default|SetisChasing true)
  (Variables|M_State|SetisGoingBase false)
  (CallFunction|SetColor))

(fn BoostActivated
  (Variables|Default|SetcanDie true)
  (Variables|Default|SetisChasing false)
  (Variables|Default|SetisRunningAway true))

(fn BoostDeactivated
  (Variables|Default|SetcanDie false)
  (Variables|Default|SetisChasing true)
  (Variables|Default|SetisRunningAway false))

(fn SetColor
  (bind _returnvalue (Math|Random|RandomFloat))
  (bind _returnvalue_2 (Math|Random|RandomFloat))
  (bind _returnvalue_3 (Math|Random|RandomFloat))
  (bind _returnvalue_4 (Math|Color|MakeColor _returnvalue_2 _returnvalue_3 _returnvalue))
  (Utilities|FlowControl|Sequence
    (:then_0
      (bind _returnvalue_5 (Rendering|Material|CreateDynamicMaterialInstance (Variables|Default|GetBody) 0 "/Game/_Main/Blueprints/Enemy/Mat_EnemySeeThrough.Mat_EnemySeeThrough" "BodyMaterialSeeThrough" :!class /Script/Engine.PrimitiveComponent))
      (Utilities|IsValid _returnvalue_5
        (:Is%20Valid
          (bind _output_get (Variables|Default|SetMaterialSeeThrough _returnvalue_5))
          (Rendering|Material|SetVectorParameterValue _output_get "Color" _returnvalue_4 :!class /Script/Engine.MaterialInstanceDynamic))))
    (:then_1
      (bind _returnvalue_6 (Rendering|Material|CreateDynamicMaterialInstance (Variables|Default|GetBody) 0 "/Game/_Main/Blueprints/Enemy/Mat_Enemy.Mat_Enemy" "BodyMaterial" :!class /Script/Engine.PrimitiveComponent))
      (Utilities|IsValid _returnvalue_6
        (:Is%20Valid
          (bind _output_get_2 (Variables|MState|SetMaterial _returnvalue_6))
          (Rendering|Material|SetVectorParameterValue _output_get_2 "Color" _returnvalue_4 :!class /Script/Engine.MaterialInstanceDynamic))))))

(fn EnableSeeThrough
  (Rendering|Material|SetMaterial (Variables|Default|GetBody) 0 (Variables|Default|GetMaterialSeeThrough)))

(fn DisableSeeThrough
  (Rendering|Material|SetMaterial (Variables|Default|GetBody) 0 (Variables|MState|GetMaterial)))