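; Base enemy Blueprint that caches shared references when play begins.
; On BeginPlay it gets the player character and game mode through message calls, storing each only if valid.
; It also records its spawn location as StartPoint, with no further behavior defined here.
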(event EventBeginPlay
  ;[1 0 0.07029] Getting references current player and gamemode
  (Utilities|FlowControl|Sequence
    (:then_0
      (bind _playerref (Class|INTPlayer|PlayerRef(Message) (Game|GetPlayerCharacter 0)))
      (Utilities|IsValid _playerref
        (:Is%20Valid
          (Variables|Reference|SetPlayer%20Ref _playerref))))
    (:then_1
      (bind _gamemode (Class|INTGamemode|GamemodeRef(Message) (Game|GetGameMode)))
      (Utilities|IsValid _gamemode
        (:Is%20Valid
          (Variables|Reference|SetGamemode _gamemode))))
    (:then_2
      (Variables|Default|SetStartPoint (Transformation|GetActorLocation)))))

(fn ConstructionScript)